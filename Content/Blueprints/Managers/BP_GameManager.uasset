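; BP_GameManager is a manager Blueprint that sets up the master HUD and drives the player's stamina.
; On BeginPlay it creates WBP_Master, passes its health and stamina sub-widgets to BPHealthComponent, then caches the ThirdPersonCharacter found in the level.
; Every Tick it polls the player's Sprinting flag and tells BPHealthComponent to decrease stamina while sprinting or increase it otherwise.
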(event EventBeginPlay
  (Utilities|FlowControl|Sequence
    (:then_0
      (bind _returnvalue (UserInterface|CreateWidget "/Game/Blueprints/Widgets/WBP_Master.WBP_Master_C" (Game|GetPlayerController 0)))
      (bind _output_get (Variables|Default|SetMasterUI _returnvalue))
      (UserInterface|Viewport|AddtoViewport _output_get 0)
      (CallFunction|SettingHealthUIRef)
      (CallFunction|SettingStaminaUIRef))
    (:then_1
      (bind _returnvalue_2 (Actor|GetActorOfClass "/Game/Player/Blueprints/ThirdPersonCharacter.ThirdPersonCharacter_C"))
      (Variables|Default|SetPlayer _returnvalue_2))))

(event EventTick
  (params (DeltaSeconds :type Float%20%28single-precision%29))
  (if (Variables|/Game/Player/Blueprints/ThirdPersonCharacter.ThirdPersonCharacter_C|GetbSprinting (Variables|Default|GetPlayer))
    (Default|DecreaseStamina (Variables|Default|GetBP_HealthComponent))
    (else
      (Default|IncreaseStamina (Variables|Default|GetBP_HealthComponent)))))

(fn ConstructionScript)

(fn SettingHealthUIRef
  (Variables|/Game/Blueprints/Components/BP_HealthComponent.BP_HealthComponent_C|SetHealthUI (Variables|Default|GetBP_HealthComponent) (Variables|/Game/Blueprints/Widgets/WBP_Master.WBP_Master_C|GetWBP_Health (Variables|Default|GetMasterUI))))

(fn SettingStaminaUIRef
  (Variables|/Game/Blueprints/Components/BP_HealthComponent.BP_HealthComponent_C|SetStaminaUI (Variables|Default|GetBP_HealthComponent) (Variables|/Game/Blueprints/Widgets/WBP_Master.WBP_Master_C|GetWBP_Stamina (Variables|Default|GetMasterUI))))