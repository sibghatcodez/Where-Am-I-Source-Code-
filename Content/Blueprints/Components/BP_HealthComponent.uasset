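; Player health and stamina component that drains health while stamina is empty.
; The health and stamina UI progress bars serve as the stored values, with getters returning each as a percent fraction and scaled to 100.
; Tick lowers health by a fixed per-frame step, without delta-time scaling.
; Stamina increase and decrease functions apply fixed, bound-checked steps but are not called within this graph.
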(event EventTick
  (params (DeltaSeconds :type Float%20%28single-precision%29))
  (bind _playerstaminainpercent (CallFunction|GetPlayerStamina))
  (if (<= _playerstaminainpercent 0.0)
    (CallFunction|DecreaseHealth)))

(fn GetPlayerHealth
  (bind _healthui (Variables|Default|GetHealthUI))
  (bind _healthbar (Variables|/Game/Blueprints/Health/WBP_Health.WBP_Health_C|GetHealthBar _healthui))
  (bind _percent (Variables|/Script/UMG.ProgressBar|GetPercent _healthbar))
  (return (* _percent 1e+02) _percent))

(fn DecreaseStamina
  (bind _staminaui (Variables|Default|GetStaminaUI))
  (bind _staminabar (Variables|/Game/Blueprints/Health/WBP_Stamina.WBP_Stamina_C|GetStaminaBar _staminaui))
  (bind _percent (Variables|/Script/UMG.ProgressBar|GetPercent _staminabar))
  (if (> _percent 0.0)
    (Progress|SetPercent _staminabar (- _percent 0.005))))

(fn IncreaseStamina
  (bind _staminaui (Variables|Default|GetStaminaUI))
  (bind _staminabar (Variables|/Game/Blueprints/Health/WBP_Stamina.WBP_Stamina_C|GetStaminaBar _staminaui))
  (bind _percent (Variables|/Script/UMG.ProgressBar|GetPercent _staminabar))
  (if (< _percent 1.0)
    (Progress|SetPercent _staminabar (+ _percent 0.00095))))

(fn GetPlayerStamina
  (bind _staminaui (Variables|Default|GetStaminaUI))
  (bind _staminabar (Variables|/Game/Blueprints/Health/WBP_Stamina.WBP_Stamina_C|GetStaminaBar _staminaui))
  (bind _percent (Variables|/Script/UMG.ProgressBar|GetPercent _staminabar))
  (return (* _percent 1e+02) _percent))

(fn DecreaseHealth
  (bind _healthui (Variables|Default|GetHealthUI))
  (bind _healthbar (Variables|/Game/Blueprints/Health/WBP_Health.WBP_Health_C|GetHealthBar _healthui))
  (bind _percent (Variables|/Script/UMG.ProgressBar|GetPercent _healthbar))
  (bind _returnvalue (- _percent 0.001))
  (if (> _percent 0.0)
    (Progress|SetPercent (Variables|/Game/Blueprints/Health/WBP_Health.WBP_Health_C|GetHealthBar (Variables|Default|GetHealthUI)) _returnvalue)
    (return _returnvalue)))