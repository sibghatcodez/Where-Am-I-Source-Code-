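; BP_ItemPlacer scatters randomly chosen items across the navigable area of the level when play begins.
; It spawns BP_Item actors in a loop driven by ItemsToPlace, each at a random navigable point within a fixed radius of the world origin.
; Each spawned item takes a random row from the DT_Items data table, which sets its static mesh and item struct.
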(event EventBeginPlay
  (CallFunction|PlaceItems (Variables|Default|GetItemsToPlace)))

(fn ConstructionScript)

(fn PlaceItems
  (params (Items%20To%20Place :type Integer))
  (for _index (range 0 Items%20To%20Place)
    (bind _random_location (CallFunction|GetRandomLocation))
    (bind _returnvalue (Game|SpawnActorfromClass "/Game/Blueprints/BP_Item.BP_Item_C" (Math|Transform|MakeTransform _random_location "0, 0, 0" "1,1,1") "Undefined" 0 0))
    (CallFunction|SetPlacedItemInformation _returnvalue)))

(fn GetRandomItem
  (bind _outrownames (DataTable|GetDataTableRowNames "/Game/Blueprints/Data/DT_Items.DT_Items"))
  (bind _returnvalue (Utilities|GetDataTableRow "/Game/Blueprints/Data/DT_Items.DT_Items" (.OutItem (Utilities|Array|Random _outrownames)))
    (:then
      (return _returnvalue))))

(fn GetRandomLocation
  (return (.RandomLocation (Class|NavigationSystemV1|GetRandomPointinNavigableRadius (Math|Vector|VectorZero) 1e+03 0 0))))

(fn SetPlacedItemInformation
  (params (Item_BP :type BP%20Item%20Object%20Reference))
  (LocalVariables|SetItem_BP_Local Item_BP)
  (bind _st_items (CallFunction|GetRandomItem))
  (Utilities|FlowControl|Sequence
    (:then_0
      ;[0.3325 0 0] Setting Mesh of our Item
      (Components|StaticMesh|SetStaticMesh (Variables|/Game/Blueprints/BP_Item.BP_Item_C|GetStaticMesh (LocalVariables|GetItem_BP_Local)) (.StaticMesh (Utilities|Struct|BreakST_Items _st_items))))
    (:then_1
      ;[0.3325 0 0] Setting The Name Of our Item
      (Variables|/Game/Blueprints/BP_Item.BP_Item_C|SetItem%20Struct (LocalVariables|GetItem_BP_Local) _st_items))))